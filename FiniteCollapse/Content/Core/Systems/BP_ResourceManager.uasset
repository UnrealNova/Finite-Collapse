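; Resource manager actor that drains four resources over time: Power, Oxygen, Cooling and Integrity.
; Each is an STResourceData struct holding current value, max value and decay rate.
; Every Tick, a separate update function per resource subtracts decay rate times world delta seconds, clamps between zero and max, and rebuilds the struct.
; The Power update also prints its current value as debug output.
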(event EventBeginPlay)

(event Collision|EventActorBeginOverlap
  (params (OtherActor :type Actor%20Object%20Reference)))

(event EventTick
  (params (DeltaSeconds :type Float%20%28single-precision%29))
  (CallFunction|UpdatePower)
  (CallFunction|UpdateOxygen)
  (CallFunction|UpdateCooling)
  (CallFunction|UpdateIntegrity))

(fn ConstructionScript)

(fn UpdatePower
  (bind _output_get (Variables|Default|SetPower (Utilities|Struct|MakeST_ResourceData (Math|Float|Clamp(Float) (- (.CurrentValue (Utilities|Struct|BreakST_ResourceData (Variables|Default|GetPower))) (* (.DecayRate (Utilities|Struct|BreakST_ResourceData (Variables|Default|GetPower))) (Utilities|Time|GetWorldDeltaSeconds))) 0.0 (.MaxValue (Utilities|Struct|BreakST_ResourceData (Variables|Default|GetPower)))) (.MaxValue (Utilities|Struct|BreakST_ResourceData (Variables|Default|GetPower))) (.DecayRate (Utilities|Struct|BreakST_ResourceData (Variables|Default|GetPower))))))
  (Development|PrintString (Utilities|String|ToString(Float) (.currentvalue _output_get))))

(fn UpdateOxygen
  (Variables|Default|SetOxygen (Utilities|Struct|MakeST_ResourceData (Math|Float|Clamp(Float) (- (.CurrentValue (Utilities|Struct|BreakST_ResourceData (Variables|Default|GetOxygen))) (* (.DecayRate (Utilities|Struct|BreakST_ResourceData (Variables|Default|GetOxygen))) (Utilities|Time|GetWorldDeltaSeconds))) 0.0 (.MaxValue (Utilities|Struct|BreakST_ResourceData (Variables|Default|GetOxygen)))) (.MaxValue (Utilities|Struct|BreakST_ResourceData (Variables|Default|GetOxygen))) (.DecayRate (Utilities|Struct|BreakST_ResourceData (Variables|Default|GetOxygen))))))

(fn UpdateCooling
  (Variables|Default|SetCooling (Utilities|Struct|MakeST_ResourceData (Math|Float|Clamp(Float) (- (.CurrentValue (Utilities|Struct|BreakST_ResourceData (Variables|Default|GetCooling))) (* (.DecayRate (Utilities|Struct|BreakST_ResourceData (Variables|Default|GetCooling))) (Utilities|Time|GetWorldDeltaSeconds))) 0.0 (.MaxValue (Utilities|Struct|BreakST_ResourceData (Variables|Default|GetCooling)))) (.MaxValue (Utilities|Struct|BreakST_ResourceData (Variables|Default|GetCooling))) (.DecayRate (Utilities|Struct|BreakST_ResourceData (Variables|Default|GetCooling))))))

(fn UpdateIntegrity
  (Variables|Default|SetIntegrity (Utilities|Struct|MakeST_ResourceData (Math|Float|Clamp(Float) (- (.CurrentValue (Utilities|Struct|BreakST_ResourceData (Variables|Default|GetIntegrity))) (* (.DecayRate (Utilities|Struct|BreakST_ResourceData (Variables|Default|GetIntegrity))) (Utilities|Time|GetWorldDeltaSeconds))) 0.0 (.MaxValue (Utilities|Struct|BreakST_ResourceData (Variables|Default|GetIntegrity)))) (.MaxValue (Utilities|Struct|BreakST_ResourceData (Variables|Default|GetIntegrity))) (.DecayRate (Utilities|Struct|BreakST_ResourceData (Variables|Default|GetIntegrity))))))